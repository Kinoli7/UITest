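; Main game player controller that creates the tile view and list menu widgets on BeginPlay.
; Debug key N and the gamepad Special Right debug key share a FlipFlop that shows or removes the list menu, switching input mode and cursor visibility with it.
; A similar toggle for the tile view menu is present but unwired, so that menu is never displayed here.
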(event EventBeginPlay
  ;[1 1 1] Widget Initialization
  (bind _returnvalue (UserInterface|CreateWidget "/Game/UI/TileView/W_TileViewMenu.W_TileViewMenu_C"))
  (Variables|Default|SetTileViewMenu _returnvalue)
  (bind _returnvalue_2 (UserInterface|CreateWidget "/Game/UI/ListMenu/W_ListMenu.W_ListMenu_C"))
  (Variables|Default|SetListMenu _returnvalue_2))

(event Input|KeyboardEvents|DebugKeyM
  (params (Key :type Key%20Structure :default "None") (ActionValue :type Input%20Action%20Value%20Structure))
  ;[1 1 1] TileView
)

(event Input|GamepadEvents|DebugKeyGamepadSpecialRight
  (params (Key :type Key%20Structure :default "None") (ActionValue :type Input%20Action%20Value%20Structure))
  (bind _self self)
  (bind _listmenu (Variables|Default|GetListMenu))
  ;[1 1 1] ListMenu
  (:Released
    (Utilities|FlowControl|FlipFlop
      (:A
        (UserInterface|Viewport|AddtoViewport _listmenu 0)
        (Input|SetInputModeGameandUI _self 0 "DoNotLock" true false)
        (Variables|Default|SetbShowMouseCursor true))
      (:B
        (Widget|RemovefromParent _listmenu)
        (Input|SetInputModeGameOnly _self false)
        (Variables|Default|SetbShowMouseCursor false)))))

(event Input|KeyboardEvents|DebugKeyN
  (params (Key :type Key%20Structure :default "None") (ActionValue :type Input%20Action%20Value%20Structure))
  (bind _self self)
  (bind _listmenu (Variables|Default|GetListMenu))
  ;[1 1 1] ListMenu
  (:Released
    (Utilities|FlowControl|FlipFlop
      (:A
        (UserInterface|Viewport|AddtoViewport _listmenu 0)
        (Input|SetInputModeGameandUI _self 0 "DoNotLock" true false)
        (Variables|Default|SetbShowMouseCursor true))
      (:B
        (Widget|RemovefromParent _listmenu)
        (Input|SetInputModeGameOnly _self false)
        (Variables|Default|SetbShowMouseCursor false)))))

(fn ConstructionScript)